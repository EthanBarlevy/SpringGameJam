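; BP_Player is a player Blueprint that lets the user drag physics objects with the mouse.
; Pressing the left button traces from the cursor, stores distance and component for movable hits, and grabs the component through a PhysicsHandle if its actor is tagged Grabbable.
; Each tick moves the handle target along the deprojected cursor ray at the stored distance, and releasing the button drops the object.
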(event `self.ReceiveTick`
  (params (DeltaSeconds :type "Float (single-precision)"))
  (bind (_worldlocation _worlddirection) (`PlayerController.DeprojectMousePositionToWorld` (`GameplayStatics.GetPlayerController` 0)))
  (`PhysicsHandleComponent.SetTargetLocation` (`self.PhysicsHandle`) (+ _worldlocation (* _worlddirection (`self.Distance`)))))

(event `Key|LeftMouseButton` :paused true
  (params (Key :type "Key Structure"))
  (bind (_worldlocation _worlddirection) (`PlayerController.DeprojectMousePositionToWorld` (`GameplayStatics.GetPlayerController` 0)))
  (:`Pressed`
    (bind (_outhit _returnvalue) (`KismetSystemLibrary.LineTraceSingle` _worldlocation (+ _worldlocation (* _worlddirection 100000.0)) "TraceTypeQuery1" true))
    (if _returnvalue
      (if (== (`SceneComponent.Mobility` (`.HitComponent` (`GameplayStatics.BreakHitResult` _outhit))) (`KismetMathLibrary.Conv_ByteToInt` (enumliteral `EComponentMobility` "Movable")))
        (bind (_bblockinghit _binitialoverlap _time _distance _location _impactpoint _normal _impactnormal _physmat _hitactor _hitcomponent) (`GameplayStatics.BreakHitResult` _outhit))
        (set `self.Distance` _distance)
        (set `self.Hit Component` _hitcomponent)
        (if (`self.ActorHasTag` _hitactor "Grabbable")
          (`PhysicsHandleComponent.GrabComponentAtLocation` (`self.PhysicsHandle`) (`self.Hit Component`) "None" _location)))))
  (:`Released`
    (set `self.Hit Component` null)
    (`PhysicsHandleComponent.ReleaseComponent` (`self.PhysicsHandle`))))

(fn `UserConstructionScript`)