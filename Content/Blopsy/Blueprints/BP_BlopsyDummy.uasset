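; BP_BlopsyDummy is a stand-in Blopsy actor that spins, blinks and is rendered in isolation by its SceneCaptureComponent2D.
; Tick rotates the Blopsy component and, through a DoOnce, sets the blink timer and limits the capture to this actor's components.
; Blink briefly swaps the Face's eye sprite material parameter, restores the default, then resets the DoOnce so the next Tick re-rolls the random interval.
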(event `self.ReceiveBeginPlay`)

(event `self.ReceiveTick`
  (params (DeltaSeconds :type "Float (single-precision)"))
  (`SceneComponent.K2_AddWorldRotation` (`self.Blopsy`) (struct :`Pitch` 1.0 :`Yaw` -3.0 :`Roll` 2.0) false false)
  (`/Engine/EditorBlueprintResources/StandardMacros.DoOnce` false :!label _label
    (:`Completed`
      (`KismetSystemLibrary.K2_SetTimerDelegate` (delegate `Blink`) (`KismetMathLibrary.RandomFloatInRange` 2.0 5.0) true)
      (`SceneCaptureComponent.ShowOnlyActorComponents` (`self.SceneCaptureComponent2D`) self false))))

(event `Blink`
  (`MeshComponent.SetScalarParameterValueOnMaterials` (`self.Face`) "EyesSpriteIDX" 1.0)
  (`KismetSystemLibrary.Delay` 0.2)
  (`MeshComponent.SetScalarParameterValueOnMaterials` (`self.Face`) "EyesSpriteIDX" (`self.DefaultEyes`))
  (goto _label :!via `Reset`))

(fn `UserConstructionScript`)