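; Blopsy is a virtual pet whose hunger, happiness and cleanliness decay every Tick, changing its mouth and eye sprites and toggling flies.
; A looping timer rolls it with velocity impulses toward Left, Center or Right points, snapping and choosing the next on arrival.
; A forward line trace bites BP_Food to restore hunger, with a chewing countdown between bites.
; Blinks run on a randomized timer, which also applies eye mood changes.
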(event `Roll_Event`
  (bind _next_location (`self.Next Location`))
  (`self.MoveTowards` _next_location)
  (if (== _next_location (`SceneComponent.K2_GetComponentLocation` (`self.Blopsy`)) :`ErrorTolerance` 10.0)
    (`self.Stop at spot` _next_location)
    (`self.Determine Next Location`)))

(event `self.ReceiveBeginPlay`
  (set `self.Next Location` (select `int` 0 :`0` (`self.Left`) :`1` (`self.Right`)))
  (`KismetSystemLibrary.K2_SetTimerDelegate` (delegate `Roll_Event`) (`KismetMathLibrary.RandomFloatInRange` 5.0 6.0) true))

(event `self.ReceiveTick`
  (params (DeltaSeconds :type "Float (single-precision)"))
  (`self.Reduce Needs` DeltaSeconds)
  (`MeshComponent.SetScalarParameterValueOnMaterials` (`self.Face`) "MouthSpriteIDX" (`self.DefaultMouth`))
  (`self.Take Bite`)
  (if (`self.IsChewing`)
    (bind _result (`/Engine/EditorBlueprintResources/StandardMacros.DecrementFloat` (`self.EatTimer`))
      (:`  `
        (if (<= _result 0.0)
          (set `self.IsChewing` false)))))
  (`/Engine/EditorBlueprintResources/StandardMacros.DoOnce` false :!label _label
    (:`Completed`
      (`KismetSystemLibrary.K2_SetTimerDelegate` (delegate `Blink`) (`KismetMathLibrary.RandomFloatInRange` 2.0 5.0) true))))

(event `Blink`
  (`MeshComponent.SetScalarParameterValueOnMaterials` (`self.Face`) "EyesSpriteIDX" 1.0)
  (`KismetSystemLibrary.Delay` 0.2)
  (`MeshComponent.SetScalarParameterValueOnMaterials` (`self.Face`) "EyesSpriteIDX" (`self.DefaultEyes`))
  (goto _label :!via `Reset`))

(fn `Determine Next Location`
  (bind _blopsy (`self.Blopsy`))
  (bind _returnvalue (`SceneComponent.K2_GetComponentLocation` _blopsy))
  (if (== (`SceneComponent.K2_GetComponentLocation` _blopsy) (`self.Left`) :`ErrorTolerance` 6.0)
    (set `self.Next Location` (`self.Center`))
    (elif (== _returnvalue (`self.Center`) :`ErrorTolerance` 6.0)
      (set `self.Next Location` (select `int` 0 :`0` (`self.Right`) :`1` (`self.Left`)))
      (elif (== _returnvalue (`self.Right`) :`ErrorTolerance` 6.0)
        (set `self.Next Location` (`self.Center`))
        (else
          (set `self.Next Location` (select `int` 0 :`0` (`self.Right`) :`1` (`self.Left`))))))))

(fn `Keep Face Up`)

(fn `MoveTowards`
  (params (Location :type "Vector Structure"))
  (bind _returnvalue (`SceneComponent.K2_GetComponentLocation` (`self.Blopsy`)))
  (`PrimitiveComponent.AddVelocityChangeImpulseAtLocation` (`self.Blopsy`) (* (- Location _returnvalue) 2.5) (- _returnvalue (0.0 0.0 -5.0)) "None"))

(fn `Reduce Needs`
  (params (DeltaTime :type "Float (double-precision)"))
  (bind _happiness (`self.Happiness`))
  (bind _hunger (`self.Hunger`))
  (set `self.Hunger` (- (`self.Hunger`) (* DeltaTime (`self.HungerRate`))))
  (set `self.Happiness` (- (`self.Happiness`) (* DeltaTime (`self.HappinessRate`))))
  (set `self.Cleanliness` (- (`self.Cleanliness`) (* DeltaTime (`self.CleanlinessRate`))))
  (`|ExecutionSequence`
    (:`then_0`
      (if (< _hunger 50.0)
        (if (< _hunger 10.0)
          (set `self.DefaultMouth` (`KismetMathLibrary.Conv_IntToDouble` (`KismetMathLibrary.RandomIntegerInRange` 5 8)))
          (else
            (set `self.DefaultMouth` 9.0)))
        (else
          (set `self.DefaultMouth` 2.0))))
    (:`then_1`
      (if (< _happiness 50.0)
        ;[0.09896 0.09896 0.09896] this isint ideal because the eyes dont update until blopsy blinks but whatever
        (if (< _happiness 10.0)
          (set `self.DefaultEyes` 5.0)
          (else
            (set `self.DefaultEyes` 3.0)))
        (else
          (set `self.DefaultEyes` 6.0))))
    (:`then_2`
      (if (< (`self.Cleanliness`) 50.0)
        (`/Engine/EditorBlueprintResources/StandardMacros.DoOnce` false :!label _label
          (:`Completed`
            (`ActorComponent.Activate` (`self.Flies`) false)))
        (else
          (`ActorComponent.Deactivate` (`self.Flies`))
          (goto _label :!via `Reset`))))))

(fn `Stop at spot`
  (params (loc :type "Vector Structure"))
  (`SceneComponent.K2_SetWorldLocationAndRotation` :`self` (`self.Blopsy`) :`NewLocation` loc :`bSweep` true))

(fn `Take Bite`
  (bind _arrow (`self.Arrow`))
  (bind _returnvalue (`SceneComponent.K2_GetComponentLocation` _arrow))
  (bind _outhit (`KismetSystemLibrary.LineTraceSingle` :`Start` _returnvalue :`End` (+ _returnvalue (* (`SceneComponent.GetForwardVector` _arrow) 200.0)) :`TraceChannel` "TraceTypeQuery1" :`bIgnoreSelf` false))
  (bind _asbp_food (cast `/Game/Blopsy/Blueprints/BP_Food` (`.HitActor` (`GameplayStatics.BreakHitResult` _outhit))))
  (if (not (`self.IsChewing`))
    (set `self.IsChewing` true)
    (set `self.EatTimer` 150.0)
    (`/Game/Blopsy/Blueprints/BP_Food.Bite` _asbp_food)
    (set `self.Hunger` (+ (`self.Hunger`) 20.0))))

(fn `UserConstructionScript`)